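; Bullet projectile actor that randomizes its launch velocity for imprecision and destroys itself on hit.
; On BeginPlay it adds normally distributed offsets along its right and forward vectors, scaled by ImprecisionMultiplier.
; NormalFloat generates those offsets with a Box-Muller transform, using log base 2 rather than natural log.
; On hit it prints the player-to-impact distance divided by 100 and draws a debug sphere.
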(event EventBeginPlay
  (bind _projectilemovement (Variables|Default|GetProjectileMovement))
  (Variables|/Script/Engine.MovementComponent|SetVelocity _projectilemovement (+ (Variables|/Script/Engine.MovementComponent|GetVelocity _projectilemovement) (* (+ (* (Transformation|GetActorRightVector) (CallFunction|NormalFloat 0.0 2e+01)) (* (Transformation|GetActorForwardVector) (CallFunction|NormalFloat 0.0 2e+01))) (Variables|Default|GetImprecisionMultiplier)))))

(event Collision|EventActorBeginOverlap
  (params (OtherActor :type Actor%20Object%20Reference)))

(event EventTick
  (params (DeltaSeconds :type Float%20%28single-precision%29)))

(event Collision|EventHit
  (params (MyComp :type Primitive%20Component%20Object%20Reference) (Other :type Actor%20Object%20Reference) (OtherComp :type Primitive%20Component%20Object%20Reference) (bSelfMoved :type Boolean) (HitLocation :type Vector :default "0, 0, 0") (HitNormal :type Vector :default "0, 0, 0") (NormalImpulse :type Vector :default "0, 0, 0") (Hit :type Hit%20Result%20Structure%20%28by%20ref%29))
  (Development|PrintString (Utilities|String|ToString(Float) (/ (Math|Vector|VectorLength (- HitLocation (Transformation|GetActorLocation (Game|GetPlayerCharacter 0)))) 1e+02)))
  (Rendering|Debug|DrawDebugSphere HitLocation 5.0 56 "(R=0.825000,G=0.012940,B=0.000000,A=1.000000)" 2e+01)
  (Actor|DestroyActor))

(fn ConstructionScript)

(fn NormalFloat
  (params (Mean :type Float%20%28single-precision%29) (Stddev :type Float%20%28single-precision%29))
  (return (+ (* (Math|Float|Sqrt (* (Math|Float|Log (Math|Random|RandomFloatinRange 0.0001 1.0) 2.0) -2.0)) Stddev (Math|Trig|Sin(Radians) (* 2.0 (Math|Trig|GetPI) (Math|Random|RandomFloatinRange 0.0001 1.0)))) Mean)))