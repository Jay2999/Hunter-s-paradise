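; Shotgun weapon Blueprint that fires a projectile with camera shake, sound, muzzle explosion effect and timeline-driven recoil on the body.
; Fire spawns the projectile at the effect's transform, then blocks refiring until a short delay ends and switches the effect off.
; Tick keeps a rolling buffer of recent barrel-tip positions, whose summed deviation from their average sets the projectile's imprecision, so barrel movement reduces accuracy.
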(event Custom|Fire
  (params (Character :type Main%20Character%20Object%20Reference))
  (bind _p_explosion_side (Variables|Default|GetP_Explosion_Side))
  (if (not (Variables|Default|GetFired))
    (Default|PlayCameraShake Character)
    (CallFunction|PlayShootAnimation)
    (Variables|Default|SetFired true)
    (Components|Activation|SetActive (Variables|Default|GetP_Explosion_Side) true false)
    (Audio|PlaySoundatLocation "/Game/Audio/AShotgunShot.AShotgunShot" (Transformation|GetActorLocation) "0, 0, 0" 1.0 1.0 0.2 0 0 0)
    (Game|SpawnActorfromClass "/Game/Blueprints/BulletProjectile.BulletProjectile_C" (Math|Transform|MakeTransform (Transformation|GetWorldLocation _p_explosion_side) (Transformation|GetWorldRotation _p_explosion_side)) "Undefined" 0 (CallFunction|GetImprecisionMultiplier) 0)
    (Utilities|FlowControl|Delay 2.0)
    (Components|Activation|SetActive (Variables|Default|GetP_Explosion_Side) false false)
    (Variables|Default|SetFired false)))

(event Custom|PlayShootAnimation
  (bind _body (Variables|Default|GetBody))
  (bind _alpha (Timeline|Timeline_0 PlayFromStart)
    (:Update
      (Transformation|SetRelativeLocation _body (Math|Vector|MakeVector (+ (* _alpha -8.0) 2e+01) 5.0 -2e+01) false false)
      (Transformation|SetRelativeRotation _body (Math|Rotator|MakeRotator (* _alpha -5.0) 0.0 -9e+01) false false))))

(event EventBeginPlay
  (Components|Activation|SetActive (Variables|Default|GetP_Explosion_Side) false false))

(event Collision|EventActorBeginOverlap
  (params (OtherActor :type Actor%20Object%20Reference)))

(event EventTick
  (params (DeltaSeconds :type Float%20%28single-precision%29))
  (bind _barreltiplocations (Variables|Default|GetBarrelTipLocations))
  (Utilities|Array|Add _barreltiplocations (Transformation|GetWorldLocation (Variables|Default|GetP_Explosion_Side)))
  (while (< 15 (Utilities|Array|Length _barreltiplocations))
    (Utilities|Array|RemoveIndex (Variables|Default|GetBarrelTipLocations))))

(fn ConstructionScript)

(fn GetImprecisionMultiplier
  (bind _barreltiplocations (Variables|Default|GetBarrelTipLocations))
  (for _array_element _barreltiplocations
    (LocalVariables|SetSumLengths (+ (Math|Vector|Distance(Vector) _array_element (Math|Vector|GetVectorArrayAverage _barreltiplocations)) (LocalVariables|GetSumLengths))))
  (return (+ (* (LocalVariables|GetSumLengths) 0.1) 1.0)))