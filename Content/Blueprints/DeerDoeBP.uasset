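; Deer doe animal character that roams the world, flees once shot and awards the player score when killed.
; A looping decision event picks short-range walking after random pauses, or fast long-range fleeing via AI MoveTo once wounded, unless hunger or tiredness flags block roaming.
; Bullet projectile hits deal fixed damage, interrupting movement with one-off hit or death animations before resuming the Animation Blueprint or destroying the corpse after a delay.
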(event Custom|Decide%20next%20action
  (params (Skip%20delay? :type Boolean))
  ;[1 1 1] Decide next action
  (if Skip%20delay?
    _
    (else
      (Utilities|FlowControl|Delay (Math|Conversions|ToFloat(Integer) (Math|Random|RandomIntegerinRange 1 5)))))
  (if (Variables|Default|GetShould%20run?)
    (CallFunction|RunAway)
    (elif (not (Variables|Default|GetIs%20hungry?))
      (if (not (Variables|Default|GetIs%20tired?))
        (CallFunction|RandomRoam)))))

(event Custom|Take%20damage
  (bind _charactermovement (Variables|Character|GetCharacterMovement))
  ;[1 1 1] Take damage
  (if (not (Variables|Damage|GetIs%20dead?))
    (bind _output_get (Variables|Damage|SetHealth (Math|Integer|Clamp(Integer) (- (Variables|Damage|GetHealth) (Variables|Damage|GetDamage)) 0 (Variables|Damage|GetMax%20health))))
    (if (== _output_get 0)
      (Components|Movement|StopMovementImmediately _charactermovement)
      (Variables|Damage|SetIs%20dead? true)
      (bind _asmain_character (Utilities|Casting|CastToMainCharacter (Game|GetPlayerCharacter 0)))
      (Default|AddScore _asmain_character 10)
      (CallFunction|PlayAnimation "/Game/AnimalVarietyPack/DeerStagAndDoe/Animations/ANIM_DeerDoe_Death.ANIM_DeerDoe_Death" false)
      (Utilities|FlowControl|Delay (Math|Conversions|ToFloat(Integer) (Math|Random|RandomIntegerinRange 60 120)))
      (Actor|DestroyActor)
      (else
        (Components|Movement|StopMovementImmediately _charactermovement)
        (CallFunction|PlayAnimation "/Game/AnimalVarietyPack/DeerStagAndDoe/Animations/ANIM_DeerDoe_GetHit.ANIM_DeerDoe_GetHit" false)
        (Variables|Default|SetShould%20run? true)
        (Utilities|FlowControl|Delay 0.7)
        (CallFunction|StopAnimation)
        (if (not (Variables|Damage|GetIs%20dead?))
          (CallFunction|DecideNextAction true))))))

(event Custom|Run%20away
  (bind _returnvalue (Transformation|GetActorLocation))
  ;[1 1 1] Run away
  (Variables|/Script/Engine.CharacterMovementComponent|SetMaxWalkSpeed (Variables|Character|GetCharacterMovement) 1.5e+03)
  (AI|AIMoveTo self (.RandomLocation (AI|Navigation|GetRandomReachablePointinRadius (+ _returnvalue (* (- _returnvalue (Transformation|GetActorLocation (Game|GetPlayerCharacter 0))) 2.0)) (Math|Random|RandomFloatinRange 2e+04 3e+04) 0 0)) 0 5.0 false
    (:OnSuccess
      (CallFunction|DecideNextAction true))))

(event Custom|Random%20roam
  ;[1 1 1] Random roam
  (Variables|/Script/Engine.CharacterMovementComponent|SetMaxWalkSpeed (Variables|Character|GetCharacterMovement) 1.5e+02)
  (AI|AIMoveTo self (.RandomLocation (AI|Navigation|GetRandomReachablePointinRadius (Transformation|GetActorLocation) 1.5e+03 0 0)) 0 5.0 false
    (:OnSuccess
      (CallFunction|DecideNextAction false))))

(event EventBeginPlay
  (CallFunction|DecideNextAction false))

(event Collision|EventHit
  (params (MyComp :type Primitive%20Component%20Object%20Reference) (Other :type Actor%20Object%20Reference) (OtherComp :type Primitive%20Component%20Object%20Reference) (bSelfMoved :type Boolean) (HitLocation :type Vector :default "0, 0, 0") (HitNormal :type Vector :default "0, 0, 0") (NormalImpulse :type Vector :default "0, 0, 0") (Hit :type Hit%20Result%20Structure%20%28by%20ref%29))
  ;[1 1 1] Projectile hit
  (Utilities|Casting|CastToBulletProjectile Other)
  (Variables|Damage|SetDamage 50)
  (CallFunction|TakeDamage))

(fn ConstructionScript)

(fn PlayAnimation
  (params (Animation :type Animation%20Asset%20Object%20Reference) (Should%20loop? :type Boolean))
  (Components|Animation|PlayAnimation (Variables|Character|GetMesh) Animation Should%20loop?))

(fn StopAnimation
  (Components|Animation|SetAnimationMode (Variables|Character|GetMesh) "AnimationBlueprint"))